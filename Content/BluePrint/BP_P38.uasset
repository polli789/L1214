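; BP_P38 is a player-controlled P-38 plane pawn that constantly moves forward along its facing.
; Pitch and Roll axes rotate it locally with frame-time scaling, and holding Left Shift raises FloatingPawnMovement max speed for a boost.
; Fire spawns a BP_Rocket at the plane's transform.
; BeginPlay registers Left and Right components with BPRotateSceneComponent; NewFunction and a disconnected offset node are unused here.
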(event EventBeginPlay
  (Utilities|Array|Add (Variables|/Game/BluePrint/BP_RotateScene_Component.BP_RotateScene_Component_C|GetSceneComponents (Variables|Default|GetBP_RotateScene_Component)) (Variables|Default|GetLeft))
  (Utilities|Array|Add (Variables|/Game/BluePrint/BP_RotateScene_Component.BP_RotateScene_Component_C|GetSceneComponents (Variables|Default|GetBP_RotateScene_Component)) (Variables|Default|GetRight)))

(event Collision|EventActorBeginOverlap
  (params (OtherActor :type Actor%20Object%20Reference)))

(event EventTick
  (params (DeltaSeconds :type Float%20%28single-precision%29))
  (Pawn|Input|AddMovementInput (Transformation|GetActorForwardVector) 1.0 false))

(event Input|ActionEvents|InputActionFire
  (params (Key :type Key%20Structure :default "None"))
  (:Pressed
    (Game|SpawnActorfromClass "/Game/BluePrint/BP_Rocket.BP_Rocket_C" (Transformation|GetActorTransform) "AlwaysSpawn" "MultiplyWithRoot" 0 0)))

(event Input|AxisEvents|InputAxisPitch
  (params (AxisValue :type Float%20%28single-precision%29))
  (Transformation|AddActorLocalRotation (Math|Rotator|MakeRotator 0.0 (* (Utilities|Time|GetWorldDeltaSeconds) (Variables|Default|GetRotateSpeed) AxisValue) 0.0) false false))

(event Input|AxisEvents|InputAxisRoll
  (params (AxisValue :type Float%20%28single-precision%29))
  (Transformation|AddActorLocalRotation (Math|Rotator|MakeRotator (* (Utilities|Time|GetWorldDeltaSeconds) (Variables|Default|GetRotateSpeed) AxisValue) 0.0 0.0) false false))

(event Input|KeyboardEvents|LeftShift
  (params (Key :type Key%20Structure :default "None"))
  (:Pressed
    (Variables|/Script/Engine.FloatingPawnMovement|SetMaxSpeed (Variables|Default|GetFloatingPawnMovement) 4e+03))
  (:Released
    (Variables|/Script/Engine.FloatingPawnMovement|SetMaxSpeed (Variables|Default|GetFloatingPawnMovement) 1.2e+03)))

(fn ConstructionScript)

(fn NewFunction
  (params (self2 :type Scene%20Component%20Object%20Reference))
  (Transformation|AddLocalRotation self2 (Math|Rotator|MakeRotator (* (Utilities|Time|GetWorldDeltaSeconds) (Variables|Default|GetSpeed)) 0.0 0.0) false false))